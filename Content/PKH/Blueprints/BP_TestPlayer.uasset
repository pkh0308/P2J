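; BP_TestPlayer is a test player Blueprint that damages passers and throws bombs.
; Anything overlapping its AttackBox that casts to PasserBase receives OnDamaged with one point of damage and the player as target.
; The Punch input spawns an enlarged BP_ThrowableBomb at ThrowDistance ahead of the player and calls ThrowBomb along the forward vector with a short delay.
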(event OnComponentBeginOverlap(AttackBox)
  (params (OverlappedComponent :type Primitive%20Component%20Object%20Reference) (OtherActor :type Actor%20Object%20Reference) (OtherComp :type Primitive%20Component%20Object%20Reference) (OtherBodyIndex :type Integer) (bFromSweep :type Boolean) (SweepResult :type Hit%20Result%20Structure%20%28by%20ref%29))
  (bind _aspasser_base (Utilities|Casting|CastToPasserBase OtherActor))
  (Class|PasserBase|OnDamaged _aspasser_base 1 self))

(event EventBeginPlay
  (|CallParentFunction) ; This node is disabled and will not be called.\nDrag off pins to build functionality.
)

(event Collision|EventActorBeginOverlap
  (params (OtherActor :type Actor%20Object%20Reference)))

(event EventTick
  (params (DeltaSeconds :type Float%20%28single-precision%29)))

(event Input|ActionEvents|InputActionPunch
  (params (Key :type Key%20Structure :default "None"))
  (:Pressed
    (bind _returnvalue (Game|SpawnActorfromClass "/Game/PKH/Blueprints/Props/BP_ThrowableBomb.BP_ThrowableBomb_C" (Math|Transform|MakeTransform (+ (Transformation|GetActorLocation) (* (Transformation|GetActorForwardVector) (Variables|Default|GetThrowDistance))) (Transformation|GetActorRotation) "1.500000,1.500000,1.500000") "Undefined" "MultiplyWithRoot" 0 0))
    (Class|ThrowableBomb|ThrowBomb _returnvalue (Transformation|GetActorForwardVector) 2.0)))

(fn ConstructionScript
  (|CallParentFunction))