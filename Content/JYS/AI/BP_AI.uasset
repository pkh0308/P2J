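; AI character that turns to face the player while its AiFSM reports an attack state.
; Tick handles the look-at rotation, and overlap with BP_PlayerZero sets IsSeeingPlayer, which a custom event clears.
; FollowPlayer is empty, and the older logic for chasing via AIMoveTo, switching to a gun montage within range and drawing a debug sphere is disconnected, so the flag drives nothing here.
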(event Custom|Follow%20Player)

(event Custom|CustomEvent
  (params (OtherActor :type Actor%20Object%20Reference))
  (Utilities|Casting|CastToBP_PlayerZero OtherActor)
  (Variables|Default|SetIsSeeingPlayer false))

(event EventBeginPlay)

(event EventTick
  (params (DeltaSeconds :type Float%20%28single-precision%29))
  (if (Variables|/Script/P2J.AIFSM|GetattackState (Variables|Default|GetaiFSM))
    (Transformation|SetActorRotation (Math|Rotator|FindLookatRotation (Transformation|GetActorLocation) (Transformation|GetActorLocation (Game|GetPlayerCharacter 0))))))

(event Collision|EventActorBeginOverlap
  (params (OtherActor :type Actor%20Object%20Reference))
  (Utilities|Casting|CastToBP_PlayerZero OtherActor)
  (Variables|Default|SetIsSeeingPlayer true))

(fn ConstructionScript)